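; LaserShooter is an actor that fires a laser along its forward vector every Tick, damaging Characters it hits.
; CastOneLaser line-traces each segment and recurses through hit actors implementing ICanLaser, which supply the next origin and direction, up to a segment cap.
; Segments are pooled LaserActors, stretched between endpoints, with unused ones hidden each frame.
; An impact particle shows at terminal hits, except on a LaserReceiver.
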(event `HideAll`
  (for (_array_element _array_index) (`self.LaserActorPool`)
    (if (>= _array_index (`self.NowUseLaserSum`))
      (`self.K2_SetActorTransform` _array_element (`KismetMathLibrary.MakeTransform` (0.0 0.0 -1000.0) (struct :`Pitch` 1.0 :`Yaw` 1.0 :`Roll` 1.0)) false false)
      (`self.SetActorHiddenInGame` _array_element true)))
  (set `self.NowUseLaserSum` 0))

(event `self.ReceiveBeginPlay`)

(event `self.ReceiveTick`
  (params (DeltaSeconds :type "Float (single-precision)"))
  (`self.CastOneLaser` (`SceneComponent.K2_GetComponentLocation` (`self.DotMesh`)) (`self.GetActorForwardVector`))
  (`self.HideAll`))

(event `CastOneLaser`
  (params (OriLocation :type "Vector Structure") (Direction :type "Vector Structure") (CastActor :type "Actor Object Reference"))
  (bind _returnvalue (+ OriLocation (* Direction 3000)))
  ;[1 1 1] 投射激光，如果实现接口则递归调用
  (bind (_outhit _returnvalue_2) (`KismetSystemLibrary.LineTraceSingle` OriLocation _returnvalue "TraceTypeQuery2" false (`|MakeArray` CastActor)))
  (bind _returnlaser (`self.GetALaser`))
  (if _returnvalue_2
    (bind (_bblockinghit _binitialoverlap _time _distance _location _impactpoint _normal _impactnormal _physmat _hitactor) (`GameplayStatics.BreakHitResult` _outhit))
    (`self.SetLaserLocation` OriLocation _location _returnlaser)
    (if (`KismetSystemLibrary.DoesImplementInterface` _hitactor "/Game/BluePrint/LaserSystem/ICanLaser.ICanLaser_C")
      (if (< (`self.NowUseLaserSum`) 10)
        (bind (_newlaserspawnlocation _newlaserspawndirection) (message `/Game/BluePrint/LaserSystem/ICanLaser.SpawnNextLaser` _hitactor _returnlaser _location))
        (`self.CastOneLaser` _newlaserspawnlocation _newlaserspawndirection _hitactor))
      (else
        (cast `/Game/BluePrint/LaserSystem/LaserReceiver` _hitactor
          (:`then`
            (`ActorComponent.SetActive` (`self.ParticleSystem`) false false))
          (:`CastFailed`
            (`self.ShowParticle` _location)
            (bind `_as角色` (cast `Character` _hitactor))
            (`GameplayStatics.ApplyDamage` `_as角色` (`self.DamagePerFrame`) null null "/Script/Engine.DamageType")))))
    (else
      (`self.SetLaserLocation` OriLocation _returnvalue _returnlaser)
      (`ActorComponent.SetActive` (`self.ParticleSystem`) false false))))

(event `SetLaserLocation`
  (params (StartLoc :type "Vector Structure") (EndLoc :type "Vector Structure") (TheLaser :type "/Game/BluePrint/LaserSystem/LaserActor Object Reference"))
  (bind _returnvalue (- EndLoc StartLoc))
  (`/Game/BluePrint/LaserSystem/LaserActor.SetLaserLenth` TheLaser (`KismetMathLibrary.VSize` _returnvalue))
  (`self.K2_SetActorLocation` TheLaser (+ StartLoc (* _returnvalue 0.5)) false false)
  (`self.K2_SetActorRotation` TheLaser (`KismetMathLibrary.MakeRotFromX` _returnvalue) false))

(event `ShowParticle`
  (params (Location :type "Vector Structure"))
  (bind _particlesystem (`self.ParticleSystem`))
  (`ActorComponent.SetActive` _particlesystem true false)
  (`SceneComponent.K2_SetWorldLocation` _particlesystem Location false false))

(fn `CallBakeLaser`
  (params (FinalLaser :type "/Game/BluePrint/LaserSystem/LaserActor Object Reference"))
  (bind _laseractorpool (`self.LaserActorPool`))
  (bind _output_get (set `self.NowUseLaserSum` (+ (`KismetArrayLibrary.Array_Find` _laseractorpool FinalLaser) 1)))
  (bind (_arrayindex _arrayelement) (`/Engine/EditorBlueprintResources/StandardMacros.ReverseForEachLoop` _laseractorpool)
    (:`LoopBody`
      (if (>= _arrayindex _output_get)
        (`self.SetActorHiddenInGame` _arrayelement true)))))

(fn `GetALaser`
  (returns (ReturnLaser :type "/Game/BluePrint/LaserSystem/LaserActor Object Reference"))
  (bind _laseractorpool (`self.LaserActorPool`))
  (bind _output_get (set `self.NowUseLaserSum` (+ (`self.NowUseLaserSum`) 1)))
  (if (> _output_get (`KismetArrayLibrary.Array_Length` _laseractorpool))
    (bind _returnvalue (`|SpawnActorFromClass` "/Game/BluePrint/LaserSystem/LaserActor.LaserActor_C" (`KismetMathLibrary.MakeTransform` (0.0 0.0 -1000.0)) "Undefined" "OverrideRootScale" null null))
    (`KismetArrayLibrary.Array_Add` (`self.LaserActorPool`) _returnvalue)
    (return _returnvalue)
    (else
      (bind _output (`|GetArrayItem` _laseractorpool (- _output_get 1)))
      (`self.SetActorHiddenInGame` _output false)
      (return _output))))

(fn `UserConstructionScript`)