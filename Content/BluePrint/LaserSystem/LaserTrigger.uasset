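; A laser-activated switch that turns a list of target actors on while beams keep hitting it, and off when they stop.
; SpawnNextLaser increments a hit counter and returns the hit location and incoming direction so the beam continues straight through.
; Tick compares the counter with its last value, treating growth as lit and a stall as released.
; A DoOnce limits activation to one call, and the mesh material shows the state.
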(event `self.ReceiveTick`
  (params (DeltaSeconds :type "Float (single-precision)"))
  (if (!= (`self.NowStatue`) 0)
    (if (> (`self.NowStatue`) (`self.PreFrameStatue`))
      (set `self.PreFrameStatue` (`self.NowStatue`))
      (`/Engine/EditorBlueprintResources/StandardMacros.DoOnce` false :!label _label
        (:`Completed`
          (for _array_element (`self.TiggerActors`)
            (`/Game/BluePrint/ButtonSystem/ICanTrigger.WhenTriggerOn` _array_element))
          (`self.OnTriggerON`)))
      (else
        (for _array_element_2 (`self.TiggerActors`)
          (`/Game/BluePrint/ButtonSystem/ICanTrigger.WhenTriggerOff` _array_element_2))
        (set `self.PreFrameStatue` 0)
        (set `self.NowStatue` 0)
        (`self.OnTriggerOff`)
        (goto _label :!via `Reset`)))))

(event `OnTriggerON`
  (`PrimitiveComponent.SetMaterial` (`self.StaticMesh`) 0 "/Game/SciFiRoomsCorridors/Materials/M_Glow02.M_Glow02"))

(event `OnTriggerOff`
  (`PrimitiveComponent.SetMaterial` (`self.StaticMesh`) 0 "/Game/StarterContent/Props/Materials/M_StatueGlass.M_StatueGlass"))

(fn `SpawnNextLaser`
  (params (IncomeLaser :type "/Game/BluePrint/LaserSystem/LaserActor Object Reference") (Location :type "Vector Structure"))
  (returns (NewLaserSpawnLocation :type "Vector Structure") (NewLaserSpawnDirection :type "Vector Structure"))
  (set `self.NowStatue` (+ (`self.NowStatue`) 1))
  (return Location (`self.GetActorForwardVector` IncomeLaser)))

(fn `UserConstructionScript`)