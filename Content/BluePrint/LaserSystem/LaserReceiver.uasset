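; LaserReceiver is a laser puzzle receiver that activates linked actors while a LaserActor overlaps its Box.
; Begin overlap calls WhenTriggerOn on every actor in TriggerActors, and end overlap calls WhenTriggerOff on them.
; RecievBegin and RecievEnd swap the ring and inner mesh materials to show whether the receiver is being hit.
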(event `self.Box.OnComponentBeginOverlap`
  (params (OverlappedComponent :type "PrimitiveComponent Object Reference") (OtherActor :type "Actor Object Reference") (OtherComp :type "PrimitiveComponent Object Reference") (OtherBodyIndex :type Integer) (bFromSweep :type Boolean) (SweepResult :type "HitResult Structure (by ref)"))
  (cast `/Game/BluePrint/LaserSystem/LaserActor` OtherActor)
  (for _array_element (`self.TriggerActors`)
    (`/Game/BluePrint/ButtonSystem/ICanTrigger.WhenTriggerOn` _array_element))
  (`self.RecievBegin`))

(event `self.Box.OnComponentEndOverlap`
  (params (OverlappedComponent :type "PrimitiveComponent Object Reference") (OtherActor :type "Actor Object Reference") (OtherComp :type "PrimitiveComponent Object Reference") (OtherBodyIndex :type Integer))
  (cast `/Game/BluePrint/LaserSystem/LaserActor` OtherActor)
  (for _array_element (`self.TriggerActors`)
    (`/Game/BluePrint/ButtonSystem/ICanTrigger.WhenTriggerOff` _array_element))
  (`self.RecievEnd`))

(event `RecievBegin`
  (`PrimitiveComponent.SetMaterial` (`self.RingMesh`) 1 "/Engine/VREditor/LaserPointer/LaserPointerMaterialInst.LaserPointerMaterialInst")
  (`PrimitiveComponent.SetMaterial` (`self.InnerMesh`) 1 "/Engine/VREditor/LaserPointer/LaserPointerMaterialInst.LaserPointerMaterialInst"))

(event `RecievEnd`
  (`PrimitiveComponent.SetMaterial` (`self.RingMesh`) 1 "/Engine/EditorMaterials/PersonaFloorMat.PersonaFloorMat")
  (`PrimitiveComponent.SetMaterial` (`self.InnerMesh`) 1 "/Game/SciFiRoomsCorridors/Materials/M_Glow02.M_Glow02"))

(fn `UserConstructionScript`)