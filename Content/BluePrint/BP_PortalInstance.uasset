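; BP_PortalInstance is a game instance Blueprint that holds the game's level order and resolves which level follows the current one.
; Init fills the Leves array with the four numbered levels followed by OverviewMap.
; GetNextLevel finds NowLevel in that array and returns the following entry, falling back to HomeMenu when the level is last or not listed.
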(event `self.ReceiveInit`
  (bind _leves (`self.Leves`))
  (`KismetArrayLibrary.Array_Add` _leves "Level1")
  (`KismetArrayLibrary.Array_Add` _leves "Level2")
  (`KismetArrayLibrary.Array_Add` _leves "Level3")
  (`KismetArrayLibrary.Array_Add` _leves "Level4")
  (`KismetArrayLibrary.Array_Add` _leves "OverviewMap"))

(fn `GetNextLevel`
  (returns (NextLevel :type String))
  (bind _leves (`self.Leves`))
  (for (_array_element _array_index) _leves
    (bind _returnvalue (+ _array_index 1))
    (if (and (> (`KismetArrayLibrary.Array_Length` _leves) _returnvalue) (`KismetStringLibrary.EqualEqual_StrStr` _array_element (`self.NowLevel`)))
      (return (`|GetArrayItem` _leves _returnvalue))))
  (return "HomeMenu"))