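; SpringBoard is an actor that flips like a springboard when anything overlaps its Box, though it applies no launch force itself.
; A timeline drives its pitch by a factor of 90 degrees, keeping the roll and yaw cached in the construction script.
; After a short delay, EndLaunch plays a second timeline for the return swing, then resets the DoOnce that blocks retriggering during the cycle.
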(event `self.Box.OnComponentBeginOverlap`
  (params (OverlappedComponent :type "PrimitiveComponent Object Reference") (OtherActor :type "Actor Object Reference") (OtherComp :type "PrimitiveComponent Object Reference") (OtherBodyIndex :type Integer) (bFromSweep :type Boolean) (SweepResult :type "HitResult Structure (by ref)"))
  (`/Engine/EditorBlueprintResources/StandardMacros.DoOnce` false :!label _label
    (:`Completed`
      (bind (_direction _time) (`Timeline|SpringBoardTimeLine` :!via `PlayFromStart`)
        (:`Update`
          (`self.K2_SetActorRelativeRotation` self (`KismetMathLibrary.MakeRotator` (.roll (`self.OriRotation`)) (* 90 _time) (.yaw (`self.OriRotation`))) false false))
        (:`Finished`
          (`KismetSystemLibrary.Delay` 0.1)
          (`self.EndLaunch`))))))

(event `EndLaunch`
  (bind (_direction _retime) (`Timeline|ReverTL` :!via `PlayFromStart`)
    (:`Update`
      (`self.K2_SetActorRelativeRotation` self (`KismetMathLibrary.MakeRotator` (.roll (`self.OriRotation`)) (* 90 _retime) (.yaw (`self.OriRotation`))) false false))
    (:`Finished`
      (goto _label :!via `Reset`))))

(fn `UserConstructionScript`
  (set `self.OriRotation` (`self.K2_GetActorRotation` self)))