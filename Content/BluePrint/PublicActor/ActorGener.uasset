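; Actor that respawn-resets an assigned HandleActor by moving it back to this actor's location when its trigger-on event fires.
; Before the move, it has the FirstPersonCharacter release that object if it is the one being held.
; OpenDoor and CloseDoor play and reverse a timeline that drives nothing, and the OpenDoor calls here are disconnected, apparently leftover door logic.
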(event `self.ReceiveBeginPlay`
  ;[1 1 1] 初始化
)

(event `RemoveFromPlayer`
  (bind _asfirst_person_character (cast `/Game/FirstPersonCPP/Blueprints/FirstPersonCharacter` (`GameplayStatics.GetPlayerPawn` 0)))
  (if (`LinkooPortalCharacter.IsActorEquelHandle` _asfirst_person_character (`self.HandleActor`))
    (`LinkooPortalCharacter.ReleaseHandleActor` _asfirst_person_character)))

(event `ResetActor`
  (bind _handleactor (`self.HandleActor`))
  ;[1 1 1] 重置位置
  (`self.RemoveFromPlayer`)
  (`/Engine/EditorBlueprintResources/StandardMacros.IsValid` _handleactor
    (:`Is Valid`
      (`self.K2_SetActorLocation` _handleactor (`self.K2_GetActorLocation`) false false))))

(event `/Game/BluePrint/ButtonSystem/ICanTrigger.WhenTriggerOn`
  (`self.ResetActor`))

(event `OpenDoor`
  (bind (_direction _relativlocation) (`Timeline|时间轴_0` :!label _label)
    (:`Finished`
      (`self.CloseDoor`))))

(event `/Game/BluePrint/ButtonSystem/ICanTrigger.WhenTriggerOff`)

(event `CloseDoor`
  (goto _label :!via `Reverse`))

(fn `UserConstructionScript`)