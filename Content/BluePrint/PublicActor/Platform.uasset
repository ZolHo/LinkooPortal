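; A trigger-driven moving platform that slides out from its start location and back.
; The trigger-on event plays a sound and runs a timeline that offsets the actor along its Arrow's forward vector by Alpha times MoveDistance, without sweeping.
; The trigger-off event reverses the timeline.
; The construction script sets the travel direction by adding MoveDirection to the Arrow's relative pitch.
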(event `self.ReceiveBeginPlay`
  (set `self.OriLocation` (`self.K2_GetActorLocation`)))

(event `/Game/BluePrint/ButtonSystem/ICanTrigger.WhenTriggerOn`
  (`GameplayStatics.PlaySoundAtLocation` "/Game/MaterialSource/Active_Sound.Active_Sound" (`self.K2_GetActorLocation`) (struct) 1.0 1.0 0.0 null null null)
  (bind (_direction _alpha) (`Timeline|时间轴_0` :!label _label)
    (:`Update`
      (`self.K2_SetActorLocation` (+ (`self.OriLocation`) (* (`SceneComponent.GetForwardVector` (`self.Arrow`)) (* _alpha (`self.MoveDistance`))))))))

(event `/Game/BluePrint/ButtonSystem/ICanTrigger.WhenTriggerOff`
  (goto _label :!via `Reverse`))

(fn `UserConstructionScript`
  (`SceneComponent.K2_AddRelativeRotation` (`self.Arrow`) (`KismetMathLibrary.MakeRotator` 0.0 (`self.MoveDirection`)) false false))