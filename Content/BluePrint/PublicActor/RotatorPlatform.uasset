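; Rotating platform actor that tilts to a target rotation while triggered and returns to its starting rotation when released.
; The construction script pitches an Arrow component by RotatorTarget, and BeginPlay caches that arrow's world rotation as the target alongside the original actor rotation.
; Trigger on/off events toggle a flag that Tick uses to ease between the two with RInterpTo.
; An older timeline-driven rotation remains but never runs.
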(event `self.ReceiveBeginPlay`
  (set `self.OriRotation` (`self.K2_GetActorRotation`))
  (set `self.Target` (`SceneComponent.K2_GetComponentRotation` (`self.Arrow`))))

(event `self.ReceiveTick`
  (params (DeltaSeconds :type "Float (single-precision)"))
  (if (`self.bStart`)
    (`self.K2_SetActorRotation` (`KismetMathLibrary.RInterpTo` (`self.K2_GetActorRotation`) (`self.Target`) DeltaSeconds 4.0))
    (else
      (`self.K2_SetActorRotation` (`KismetMathLibrary.RInterpTo` (`self.K2_GetActorRotation`) (`self.OriRotation`) DeltaSeconds 4.0)))))

(event `/Game/BluePrint/ButtonSystem/ICanTrigger.WhenTriggerOn`
  (set `self.bStart` true))

(event `/Game/BluePrint/ButtonSystem/ICanTrigger.WhenTriggerOff`
  (set `self.bStart` false))

(fn `UserConstructionScript`
  (`SceneComponent.K2_AddRelativeRotation` (`self.Arrow`) (`KismetMathLibrary.MakeRotator` 0.0 (`self.RotatorTarget`)) false false))