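; ActorSetter is a placeable mover that slides an assigned HandleActor back and forth along a track while triggered.
; The construction script sizes the Left/Right markers and cube from DoorLenth.
; BeginPlay places HandleActor above the setter and derives a per-tick step from markers, DoorLenth and CycleTime.
; Tick counts frames to reverse direction, assuming 60 fps without delta time; trigger events toggle motion, playing a sound on activation.
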(event `self.ReceiveBeginPlay`
  (bind (_returnvalue_x _returnvalue_y _returnvalue_z) (`KismetMathLibrary.BreakVector` (`self.K2_GetActorLocation`)))
  (bind _handleactor (`self.HandleActor`))
  (`/Engine/EditorBlueprintResources/StandardMacros.IsValid` _handleactor
    (:`Is Valid`
      (`self.K2_SetActorLocation` _handleactor (`KismetMathLibrary.MakeVector` _returnvalue_x _returnvalue_y (+ _returnvalue_z 150.0)) false false)
      (`self.CaculMovePreTick`))))

(event `self.ReceiveTick`
  (params (DeltaSeconds :type "Float (single-precision)"))
  (bind _handleactor (`self.HandleActor`))
  (bind _movedirection (`self.MoveDirection`))
  (bind _returnvalue (`self.K2_GetActorLocation` _handleactor))
  (if (`self.bTrigger`)
    (`/Engine/EditorBlueprintResources/StandardMacros.IsValid` _handleactor
      (:`Is Valid`
        (if (`self.NowDirect`)
          (set `self.times` (+ (`self.times`) 1))
          (`self.K2_SetActorLocation` _handleactor (+ _returnvalue _movedirection) false false)
          (if (>= (`self.times`) (`KismetMathLibrary.FTrunc` (* 60 (`self.CycleTime`))))
            (set `self.NowDirect` (not (`self.NowDirect`)) :!label _label))
          (else
            (set `self.times` (+ (`self.times`) -1))
            (`self.K2_SetActorLocation` _handleactor (- _returnvalue _movedirection) false false)
            (if (<= (`self.times`) (`KismetMathLibrary.FTrunc` (* -60 (`self.CycleTime`))))
              (goto _label))))))))

(event `CaculMovePreTick`
  (bind _output_get (set `self.MovePerTick` (/ (- (`self.DoorLenth`) 40.0) (* 60 (`self.CycleTime`)))))
  (set `self.MoveDirection` (* (`KismetMathLibrary.Normal` (- (`SceneComponent.K2_GetComponentLocation` (`self.Left`)) (`SceneComponent.K2_GetComponentLocation` (`self.Right`)))) _output_get)))

(event `/Game/BluePrint/ButtonSystem/ICanTrigger.WhenTriggerOff`
  (set `self.bTrigger` false))

(event `/Game/BluePrint/ButtonSystem/ICanTrigger.WhenTriggerOn`
  (`GameplayStatics.PlaySoundAtLocation` "/Game/MaterialSource/Active_Sound.Active_Sound" (`self.K2_GetActorLocation`) (struct) 1.0 1.0 0.0 null null null)
  (set `self.bTrigger` true))

(fn `UserConstructionScript`
  (bind _doorlenth (`self.DoorLenth`))
  (`SceneComponent.K2_SetRelativeLocation` (`self.Left`) (`KismetMathLibrary.MakeVector` 0.0 (* -1 _doorlenth)) false false)
  (`SceneComponent.K2_SetRelativeLocation` (`self.Right`) (`KismetMathLibrary.MakeVector` 0.0 _doorlenth) false false)
  (`SceneComponent.SetRelativeScale3D` (`self.Cube`) (`KismetMathLibrary.MakeVector` 0.2 (/ _doorlenth 50.0) 3.0)))