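; TriggerButton is a pressure button that switches linked actors on and off as something enters or leaves its Box trigger.
; Begin and end overlap call WhenTriggerOn or WhenTriggerOff on each valid entry in TiggerActors, with no filtering or counting of overlaps.
; A timeline sinks OuterMesh slightly from the location cached in the Construction Script, and reverses to raise it on release.
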(event `self.Box.OnComponentBeginOverlap`
  (params (OverlappedComponent :type "PrimitiveComponent Object Reference") (OtherActor :type "Actor Object Reference") (OtherComp :type "PrimitiveComponent Object Reference") (OtherBodyIndex :type Integer) (bFromSweep :type Boolean) (SweepResult :type "HitResult Structure (by ref)"))
  (for _array_element (`self.TiggerActors`)
    (`/Engine/EditorBlueprintResources/StandardMacros.IsValid` (`KismetSystemLibrary.Conv_InterfaceToObject` _array_element)
      (:`Is Valid`
        (`/Game/BluePrint/ButtonSystem/ICanTrigger.WhenTriggerOn` _array_element))))
  (`self.ButtonOn`))

(event `self.Box.OnComponentEndOverlap`
  (params (OverlappedComponent :type "PrimitiveComponent Object Reference") (OtherActor :type "Actor Object Reference") (OtherComp :type "PrimitiveComponent Object Reference") (OtherBodyIndex :type Integer))
  (for _array_element (`self.TiggerActors`)
    (`/Engine/EditorBlueprintResources/StandardMacros.IsValid` (`KismetSystemLibrary.Conv_InterfaceToObject` _array_element)
      (:`Is Valid`
        (`/Game/BluePrint/ButtonSystem/ICanTrigger.WhenTriggerOff` _array_element))))
  (`self.ButtonOff`))

(event `ButtonOn`
  (bind (_direction _default) (`Timeline|AnimTimeLine` :!label _label)
    (:`Update`
      (`SceneComponent.K2_SetRelativeLocation` (`self.OuterMesh`) (+ (`self.DefaultLocation`) (`KismetMathLibrary.MakeVector` 0.0 0.0 (* -5 _default))) false false))))

(event `ButtonOff`
  (goto _label :!via `Reverse`))

(fn `UserConstructionScript`
  (set `self.DefaultLocation` (`SceneComponent.RelativeLocation` (`self.OuterMesh`))))