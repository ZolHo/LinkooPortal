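; LightLine is a spline-based light strip in the button system that lights up progressively when triggered.
; The Construction Script places shadowless static meshes at MeshGap intervals along the spline, stores them in MeshPtrs and derives UnitTime from their count.
; Trigger-on runs a timeline that swaps each mesh's second material to glow in sequence, using UnitTime as the step.
; Trigger-off restores grey on all meshes at once and stops the timeline.
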(event `/Game/BluePrint/ButtonSystem/ICanTrigger.WhenTriggerOn`
  (bind _output_get (set `self.NowDealIdx` 0))
  (bind (_direction _time) (`Timeline|时间轴_0` :!via `PlayFromStart` :!label _label)
    (:`Update`
      (if (> _time (* _output_get (`self.UnitTime`)))
        (`PrimitiveComponent.SetMaterial` (`|GetArrayItem` (`self.MeshPtrs`) _output_get) 1 "/Game/SciFiRoomsCorridors/Materials/M_Glow02.M_Glow02")
        (set `self.NowDealIdx` (+ _output_get 1))))))

(event `/Game/BluePrint/ButtonSystem/ICanTrigger.WhenTriggerOff`
  (bind (_arrayindex _arrayelement) (`/Engine/EditorBlueprintResources/StandardMacros.ReverseForEachLoop` (`self.MeshPtrs`))
    (:`LoopBody`
      (`PrimitiveComponent.SetMaterial` _arrayelement 1 "/Engine/EditorMeshes/ColorCalibrator/M_GreyBall.M_GreyBall"))
    (:`Completed`
      (goto _label :!via `Stop`))))

(fn `UserConstructionScript`
  (bind _spline (`self.Spline`))
  (for _index (range (+ (`KismetMathLibrary.Conv_Int64ToInt` (- (`KismetMathLibrary.FFloor64` (/ (`SplineComponent.GetSplineLength` (`self.Spline`)) (`self.MeshGap`))) 1)) 1))
    (bind _returnvalue (`AddComponent|NODE_AddStaticMeshComponent-0` :`bManualAttachment` true))
    (`SceneComponent.K2_AttachToComponent` _returnvalue _spline "None" "KeepRelative" "KeepRelative" "KeepRelative" true)
    (`PrimitiveComponent.SetCastShadow` _returnvalue false)
    (bind _returnvalue_2 (* _index (`self.MeshGap`)))
    (`SceneComponent.K2_SetWorldLocation` _returnvalue (`SplineComponent.GetLocationAtDistanceAlongSpline` _spline _returnvalue_2 "World") false false)
    (`SceneComponent.K2_SetWorldRotation` _returnvalue (`SplineComponent.GetRotationAtDistanceAlongSpline` _spline _returnvalue_2 "World") false false)
    (`KismetArrayLibrary.Array_Add` (`self.MeshPtrs`) _returnvalue))
  (bind _output_get (set `self.MeshSum` (`KismetArrayLibrary.Array_Length` (`self.MeshPtrs`))))
  (set `self.UnitTime` (/ 1.0 (`KismetMathLibrary.Conv_IntToDouble` _output_get))))