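; Double sliding door Blueprint in the button system that opens and closes through overridden BeginOpen and EndOpen events.
; The construction script caches the relative locations of the Left and Right panels as their default positions.
; BeginOpen plays a timeline that slides the panels in opposite directions along local Y from those defaults, and EndOpen reverses it to close them.
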(event `self.BeginOpen`
  ;[1 1 1] 重载父类
  (bind (_direction _default) (`Timeline|OpenDoorTL` :!label _label)
    (:`Update`
      (`SceneComponent.K2_SetRelativeLocation` (`self.Left`) (- (`self.DefaultLeftLocation`) (`KismetMathLibrary.MakeVector` 0.0 (* -100 _default))) false false)
      (`SceneComponent.K2_SetRelativeLocation` (`self.Right`) (- (`self.DefaultRightLocation`) (`KismetMathLibrary.MakeVector` 0.0 (* 100 _default))) false false))))

(event `self.EndOpen`
  ;[1 1 1] 重载父类
  (goto _label :!via `Reverse`))

(fn `UserConstructionScript`
  (set `self.DefaultLeftLocation` (`SceneComponent.RelativeLocation` (`self.Left`)))
  (set `self.DefaultRightLocation` (`SceneComponent.RelativeLocation` (`self.Right`))))