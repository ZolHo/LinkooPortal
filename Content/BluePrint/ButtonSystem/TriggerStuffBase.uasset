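; TriggerStuffBase is a base Blueprint in the button system for objects that open when enough triggers are on.
; WhenTriggeron and WhenTriggerOff raise and lower the NowTriggerOn count and compare it to NeedTriggerOn, calling BeginOpen at or above the threshold and EndOpen below it.
; BeginOpen and EndOpen are empty here, and either can fire repeatedly because the checks test the current count rather than a threshold crossing.
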(event `/Game/BluePrint/ButtonSystem/ICanTrigger.WhenTriggerOn`
  (bind _output_get (set `self.NowTriggerOn` (+ (`self.NowTriggerOn`) 1)))
  (if (>= _output_get (`self.NeedTriggerOn`))
    (`self.BeginOpen`)))

(event `/Game/BluePrint/ButtonSystem/ICanTrigger.WhenTriggerOff`
  (bind _output_get (set `self.NowTriggerOn` (- (`self.NowTriggerOn`) 1)))
  (if (< _output_get (`self.NeedTriggerOn`))
    (`self.EndOpen`)))

(event `BeginOpen`)

(event `EndOpen`)

(fn `UserConstructionScript`)