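; BP_LightCourrier is a main menu actor that moves its static mesh repeatedly between two tagged points in the level.
; On BeginPlay it stores the locations of the first actors tagged A and B.
; A timeline lerps the mesh from A to B, and an 8-second Delay on its update pin calls Movements again to restart the run from A.
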(event `self.ReceiveBeginPlay`
  (bind _outactors (`GameplayStatics.GetAllActorsWithTag` (`self.A`)))
  (set `self.Location A` (`self.K2_GetActorLocation` (`|GetArrayItem` _outactors)))
  (bind _outactors_2 (`GameplayStatics.GetAllActorsWithTag` (`self.B`)))
  (set `self.Location B` (`self.K2_GetActorLocation` (`|GetArrayItem` _outactors_2)))
  (`self.Movements`))

(event `Movements`
  (bind (_direction _alpha) (`Timeline|MoveTimeline` :!via `PlayFromStart`)
    (:`Update`
      (`SceneComponent.K2_SetWorldLocation` (`self.StaticMesh`) (`KismetMathLibrary.VLerp` (`self.Location A`) (`self.Location B`) _alpha) false false)
      (`KismetSystemLibrary.Delay` 8.0)
      (`self.Movements`))))

(fn `UserConstructionScript`)